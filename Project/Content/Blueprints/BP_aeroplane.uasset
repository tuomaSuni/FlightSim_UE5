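; Aeroplane Blueprint that animates a plane's moving parts on a PoseableMesh while its SpringArm slowly rotates.
; Each Tick adds a fixed step to the SpringArm's local rotation and to the Propeller bone's component-space roll, so both speeds depend on frame rate.
; Flap_L and Flap_R pitch together on a slow sine wave of game time, set directly on the bones in component space.
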(event `self.ReceiveTick`
  (params (DeltaSeconds :type "Float (single-precision)"))
  (bind _poseablemesh (`self.PoseableMesh`))
  (bind _returnvalue (+ (* (`KismetMathLibrary.Sin` (+ (* (`KismetSystemLibrary.GetGameTimeInSeconds`) 0.33) 4.712385)) 20.0) 20.0))
  (`SceneComponent.K2_AddLocalRotation` (`self.SpringArm`) (struct :`Yaw` 0.37) false false)
  (bind _returnvalue_2 (`PoseableMeshComponent.GetBoneRotationByName` _poseablemesh "Propeller" "ComponentSpace"))
  (`PoseableMeshComponent.SetBoneRotationByName` _poseablemesh "Propeller" (`KismetMathLibrary.MakeRotator` (+ (.roll _returnvalue_2) 6.0)) "ComponentSpace")
  (`PoseableMeshComponent.SetBoneRotationByName` _poseablemesh "Flap_L" (`KismetMathLibrary.MakeRotator` 0.0 _returnvalue) "ComponentSpace")
  (`PoseableMeshComponent.SetBoneRotationByName` _poseablemesh "Flap_R" (`KismetMathLibrary.MakeRotator` 0.0 _returnvalue) "ComponentSpace"))

(fn `UserConstructionScript`)